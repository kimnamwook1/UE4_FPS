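; BP_AISpawner is an AI spawner for the shooting game that creates BP_AI pawns running the BT_A behavior tree.
; On BeginPlay it caches BP_ShootingGameMode and starts a two-second timer.
; Each tick of that timer compares AIAlive to AIMax, spawns at a navigable point near itself and increments the game mode's count.
; The timer re-arms only after a spawn, so the loop stops at the cap.
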(event EventBeginPlay
  (bind _asbp_shooting_game_mode (Utilities|Casting|CastToBP_ShootingGameMode (Game|GetGameMode)))
  (Variables|Default|SetShootingGM_REF _asbp_shooting_game_mode)
  (Utilities|Time|SetTimerbyFunctionName 0 "NoticeToGM" 2.0))

(fn ConstructionScript)

(fn SpawnAI
  (bind _randomlocation (Class|NavigationSystemV1|GetRandomLocationinNavigableRadius (Transformation|GetActorLocation) 1e+01 0 0))
  (AI|SpawnAIFromClass "/Game/ShootingGame/AI/AI_Blueprint/BP_AI.BP_AI_C" "/Game/ShootingGame/AI/AI_BT/BT_A.BT_A" (Math|Vector|MakeVector (.x _randomlocation) (.y _randomlocation) (.z (Transformation|GetActorLocation))) "0, 0, 0" false 0))

(fn NoticetoGM
  (bind _shootinggm_ref (Variables|Default|GetShootingGM_REF))
  (if (< (Variables|/Game/ShootingGame/GameMode/BP_ShootingGameMode.BP_ShootingGameMode_C|GetAI_Alive _shootinggm_ref) (Variables|/Game/ShootingGame/GameMode/BP_ShootingGameMode.BP_ShootingGameMode_C|GetAI_Max _shootinggm_ref))
    (CallFunction|SpawnAI)
    (Default|IncreaseAI _shootinggm_ref)
    (Utilities|Time|SetTimerbyFunctionName 0 "NoticeToGM" 2.0)))