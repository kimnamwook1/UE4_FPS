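; Lobby HUD for the shooting game that shows the lobby widget and keeps its player list current.
; On BeginPlay it creates the widget, switches to UI-only input and shows the mouse cursor.
; BindPlayerState subscribes to a player state's name-change dispatcher and triggers an immediate refresh, with a debug print.
; Name changes update the player list, retrying on a short timer until the widget is valid.
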(event EventBeginPlay
  (bind _returnvalue (Game|GetPlayerController 0))
  (bind _returnvalue_2 (UserInterface|CreateWidget "/Game/ShootingGame/Widget/Lobby/LobbyHUDWidget.LobbyHUDWidget_C"))
  (bind _output_get (Variables|Default|SetHUDWidget _returnvalue_2))
  (UserInterface|Viewport|AddtoViewport _output_get 0)
  (Input|SetInputModeUIOnly _returnvalue 0 "DoNotLock")
  (Variables|/Script/Engine.PlayerController|SetbShowMouseCursor _returnvalue true))

(fn ConstructionScript)

(fn BindPlayerState
  (params (PlayerState :type BP%20Lobby%20Player%20State%20Object%20Reference))
  (EventDispatchers|BindEventtoEventDispatcherChangeName PlayerState (EventDispatchers|CreateEvent :!event EventChangeName))
  (Development|PrintString "Bind Player State" true true "(R=0.000000,G=0.660000,B=1.000000,A=1.000000)" 6e+01)
  (CallFunction|EventChangeName))

(fn EventChangeName
  (params (NewName :type String))
  (CallFunction|RFChangeName))

(fn RFChangeName
  (bind _hudwidget (Variables|Default|GetHUDWidget))
  (Utilities|IsValid _hudwidget
    (:Is%20Valid
      (Default|UpdatePlayerList _hudwidget))
    (:Is%20Not%20Valid
      (Utilities|Time|SetTimerbyFunctionName 0 "RF_ChangeName" 0.1))))