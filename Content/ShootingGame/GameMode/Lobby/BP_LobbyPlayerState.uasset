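; BP_LobbyPlayerState is the lobby PlayerState that holds a player's Name and announces changes to it.
; On BeginPlay it hands itself to the first player controller's BP_LobbyHUD through BindPlayerState, printing an error if the cast fails.
; SetName writes Name, and its OnRep handler prints the value and fires the ChangeName dispatcher so bound listeners can react.
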(event EventBeginPlay
  (CallFunction|InitBind))

(event EventTick
  (params (DeltaSeconds :type Float%20%28single-precision%29)))

(fn ConstructionScript)

(fn OnRepName
  (Development|PrintString (Utilities|String|Append "On Rep Name : " (Variables|Default|GetName)) true true "(R=0.000000,G=0.660000,B=1.000000,A=1.000000)" 6e+01)
  (Default|CallEventDispatcherChangeName (Variables|Default|GetName)))

(fn SetName
  (params (Name :type String))
  (Variables|Default|SetName Name))

(fn InitBind
  (bind _asbp_lobby_hud (Utilities|Casting|CastToBP_LobbyHUD (HUD|GetHUD (Game|GetPlayerController 0)))
    (:then
      (Default|BindPlayerState _asbp_lobby_hud self))
    (:CastFailed
      (Development|PrintString "BP_Lobby HUD Test Fail" true true "(R=1.000000,G=0.027049,B=0.035007,A=1.000000)" 6e+01))))